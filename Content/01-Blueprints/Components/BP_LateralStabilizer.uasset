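; BP_LateralStabilizer is a component that reduces sideways sliding on a physics-driven vehicle.
; On BeginPlay it caches the owner's root primitive, clearing the reference if that root does not simulate physics.
; Each tick it projects the linear velocity onto the body's right vector and applies an opposing mass-dependent force, scaled by ReduceLateralVelocity, to damp lateral drift.
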(event `self.ReceiveBeginPlay`
  (bind _asprimitive_component (cast `PrimitiveComponent` (`Actor.RootComponent` (`self.GetOwner`))))
  (bind _output_get (set `self.RefToVehicule` _asprimitive_component))
  (if (not (`SceneComponent.IsSimulatingPhysics` _output_get "None"))
    (set `self.RefToVehicule` null)))

(event `self.ReceiveTick`
  (params (DeltaSeconds :type "Float (single-precision)"))
  (bind _reftovehicule (`self.RefToVehicule`))
  (bind _reftovehicule_2 (`self.RefToVehicule`)
    (:`then`
      (bind _returnvalue (`PrimitiveComponent.GetPhysicsLinearVelocity` _reftovehicule_2 "None"))
      (`PrimitiveComponent.AddForce` _reftovehicule (* (* (`KismetMathLibrary.Dot_VectorVector` _returnvalue (`SceneComponent.GetRightVector` _reftovehicule_2)) -1.0 (`self.ReduceLateralVelocity`)) (`SceneComponent.GetRightVector` _reftovehicule)) "None" false))
    (:`else`)))