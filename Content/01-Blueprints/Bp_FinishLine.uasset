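; Finish line trigger actor that ends a run when the BP_Hover vehicle overlaps its box.
; On overlap it disables the player's input, removes the hover's post-process and slows global time for a slow-motion finish.
; It plays the S_FadeOutExit level sequence, waits briefly, then restores normal time and opens the main menu level.
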(event `self.Box.OnComponentBeginOverlap`
  (params (OverlappedComponent :type "PrimitiveComponent Object Reference") (OtherActor :type "Actor Object Reference") (OtherComp :type "PrimitiveComponent Object Reference") (OtherBodyIndex :type Integer) (bFromSweep :type Boolean) (SweepResult :type "HitResult Structure (by ref)"))
  ;[1 1 1] Slow Time + Back Main Menu
  (bind _asbp_hover (cast `/Game/01-Blueprints/BP_Hover` OtherActor))
  (`self.DisableInput` _asbp_hover (`GameplayStatics.GetPlayerController` 0))
  (bind _returnvalue (`GameplayStatics.GetActorOfClass` "/Game/01-Blueprints/BP_Hover.BP_Hover_C"))
  (`/Game/01-Blueprints/BP_Hover.Remove PostProcess` _returnvalue)
  (`GameplayStatics.SetGlobalTimeDilation` 0.25)
  (bind (_outactor _returnvalue_2) (`LevelSequencePlayer.CreateLevelSequencePlayer` "/Game/06-Sequencer/S_FadeOutExit.S_FadeOutExit"))
  (`MovieSceneSequencePlayer.Play` _returnvalue_2)
  (`KismetSystemLibrary.Delay` 2.0)
  (`GameplayStatics.SetGlobalTimeDilation` 1.0)
  (`GameplayStatics.OpenLevelBySoftObjectPtr` "/Game/02-Maps/L_MainMenu.L_MainMenu"))

(fn `UserConstructionScript`)